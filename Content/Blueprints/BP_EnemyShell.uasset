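; Enemy shell character that charges toward the player while they are inside its detection sphere.
; While the player is detected, Tick drives repeated forward launches and a DoOnce that snaps yaw to the player, re-armed after a delay so the heading updates only periodically.
; Capsule hits on actors without the Landscape tag zero its movement velocity.
; Debug prints show detection, the stored player position and hit actors.
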(event OnComponentBeginOverlap(DetectionSphere)
  (params (OverlappedComponent :type Primitive%20Component%20Object%20Reference) (OtherActor :type Actor%20Object%20Reference) (OtherComp :type Primitive%20Component%20Object%20Reference) (OtherBodyIndex :type Integer) (bFromSweep :type Boolean) (SweepResult :type Hit%20Result%20Structure%20%28by%20ref%29))
  ;[1 0.4248 0.1197] Player Detection Zone
  (if (== OtherActor (Game|GetPlayerCharacter 0))
    (Variables|Default|SetPlayerDetected? true)))

(event OnComponentEndOverlap(DetectionSphere)
  (params (OverlappedComponent :type Primitive%20Component%20Object%20Reference) (OtherActor :type Actor%20Object%20Reference) (OtherComp :type Primitive%20Component%20Object%20Reference) (OtherBodyIndex :type Integer))
  ;[1 0.4248 0.1197] Player Detection Zone
  (if (== OtherActor (Game|GetPlayerCharacter 0))
    (Variables|Default|SetPlayerDetected? false)))

(event OnComponentHit(CapsuleComponent)
  (params (HitComponent :type Primitive%20Component%20Object%20Reference) (OtherActor :type Actor%20Object%20Reference) (OtherComp :type Primitive%20Component%20Object%20Reference) (NormalImpulse :type Vector :default "0, 0, 0") (Hit :type Hit%20Result%20Structure%20%28by%20ref%29))
  ;[1 0.889 0.04791] Hits something
  (if (not (Actor|ActorHasTag OtherActor "Landscape"))
    (Development|PrintString (Utilities|GetDisplayName OtherActor) true true "(R=1.000000,G=0.803265,B=0.000000,A=1.000000)" 2.0 "5843")
    (CallFunction|EnemyObstacleStop)))

(event Custom|MovementFinished
  (bind _returnvalue (Transformation|GetActorLocation))
  (bind _returnvalue_2 (Game|GetPlayerCharacter 0))
  (bind _returnvalue_3 (Transformation|GetActorLocation _returnvalue_2))
  (bind _returnvalue_4 (Math|Rotator|FindLookatRotation _returnvalue _returnvalue_3))
  ;[0.2235 0.9103 1] Character Rotates
  (Utilities|FlowControl|DoOnce false) ; enters at Reset
)

(event EventTick
  (params (DeltaSeconds :type Float%20%28single-precision%29))
  (bind _returnvalue (Transformation|GetActorLocation))
  (bind _returnvalue_2 (Game|GetPlayerCharacter 0))
  (bind _returnvalue_3 (Transformation|GetActorLocation _returnvalue_2))
  (bind _returnvalue_4 (Math|Rotator|FindLookatRotation _returnvalue _returnvalue_3))
  (if (Variables|Default|GetPlayerDetected?)
    (Development|PrintString "Player Detected" true true "(R=0.450309,G=0.000000,B=1.000000,A=1.000000)" 2.0 "333")
    (Utilities|FlowControl|Sequence
      (:then_0
        ;[0.2235 0.9103 1] Character Rotates
        (Utilities|FlowControl|DoOnce false
          (:Completed
            (Variables|Default|SetPlayerPosition (Transformation|GetActorLocation (Game|GetPlayerCharacter 0)))
            (Transformation|SetActorRotation (Math|Rotator|MakeRotator (.roll _returnvalue_4) 0.0 (.yaw _returnvalue_4))))))
      (:then_1
        (Utilities|FlowControl|Delay 0.0)
        (Development|PrintText (Utilities|Text|FormatText "Destination {pos}" (Utilities|Text|ToText(String) (Variables|Default|GetPlayerPosition))) true true "(R=0.733501,G=1.000000,B=0.207101,A=1.000000)" 15.0 "848")
        ;[0.141 0.4403 1] Character Moves towards the Player
        (Character|LaunchCharacter (* (Math|Vector|GetForwardVector (Transformation|GetActorRotation)) 75.0) false false)
        (Utilities|FlowControl|Delay 2.0)
        (CallFunction|MovementFinished)))))

(fn ConstructionScript)

(fn EnemyObstacleStop
  (Variables|/Script/Engine.MovementComponent|SetVelocity (Variables|Character|GetCharacterMovement) "0, 0, 0"))