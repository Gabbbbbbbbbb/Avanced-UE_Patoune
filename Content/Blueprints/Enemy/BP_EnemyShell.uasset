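; Shell enemy that detects the player, dashes at them in repeated launches and dies when they overlap its KillBox.
; Detection shows an exclamation mark, Tick drives the dash, and MovementFinished re-aims after a delay.
; Player hits knock them back and either drain score by timer or trigger the no-coin state; other obstacles make it recoil and roll.
; A Niagara export callback turns fallen-coin particles into BP_Coin pickups.
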(event OnComponentBeginOverlap(KillBox)
  (params (OverlappedComponent :type Primitive%20Component%20Object%20Reference) (OtherActor :type Actor%20Object%20Reference) (OtherComp :type Primitive%20Component%20Object%20Reference) (OtherBodyIndex :type Integer) (bFromSweep :type Boolean) (SweepResult :type Hit%20Result%20Structure%20%28by%20ref%29))
  ;[1 1 1] Called if the player jumps on  the lower half of the enemy
  (if (== OtherActor (Game|GetPlayerCharacter 0))
    (Character|LaunchCharacter (Game|GetPlayerCharacter 0) (Math|Vector|MakeVector 0.0 0.0 (* (.z (Variables|/Script/Engine.MovementComponent|GetVelocity (Variables|/Script/Engine.Character|GetCharacterMovement (Variables|Default|GetAs%20PC%20Test)))) 5e+02)) false false)
    (Utilities|FlowControl|Delay 0.2)
    (Actor|DestroyActor)))

(event OnComponentBeginOverlap(DetectionSphere)
  (params (OverlappedComponent :type Primitive%20Component%20Object%20Reference) (OtherActor :type Actor%20Object%20Reference) (OtherComp :type Primitive%20Component%20Object%20Reference) (OtherBodyIndex :type Integer) (bFromSweep :type Boolean) (SweepResult :type Hit%20Result%20Structure%20%28by%20ref%29))
  ;[1 0.4248 0.1197] Player Detection Zone
  (if (== OtherActor (Game|GetPlayerCharacter 0))
    (Variables|Default|SetPlayerDetected? true)
    (Rendering|SetVisibility (Variables|Default|GetExclamationMark) true false)))

(event OnComponentEndOverlap(DetectionSphere)
  (params (OverlappedComponent :type Primitive%20Component%20Object%20Reference) (OtherActor :type Actor%20Object%20Reference) (OtherComp :type Primitive%20Component%20Object%20Reference) (OtherBodyIndex :type Integer))
  ;[1 0.4248 0.1197] Player Detection Zone
  (if (== OtherActor (Game|GetPlayerCharacter 0))
    _))

(event OnComponentHit(CapsuleComponent)
  (params (HitComponent :type Primitive%20Component%20Object%20Reference) (OtherActor :type Actor%20Object%20Reference) (OtherComp :type Primitive%20Component%20Object%20Reference) (NormalImpulse :type Vector :default "0, 0, 0") (Hit :type Hit%20Result%20Structure%20%28by%20ref%29))
  (bind _capsulecomponent (Variables|Collision|GetCapsuleComponent))
  (bind _niagaracoinfalloff (Variables|Default|GetNiagaraCoinFallOff))
  (bind _returnvalue (Transformation|GetWorldRotation _capsulecomponent))
  (bind _returnvalue_2 (Math|Vector|GetForwardVector _returnvalue))
  (bind _returnvalue_3 (* _returnvalue_2 1e+03))
  ;[1 0.889 0.04791] Hits something
  (if (Actor|ActorHasTag OtherActor "Landscape")
    (CallFunction|MovementFinished)
    (else
      (Development|PrintString (Utilities|GetDisplayName OtherActor) true true "(R=0.957051,G=1.000000,B=0.989953,A=1.000000)" 0.2 "5843")
      (Variables|Default|SetCanDash? false)
      (if (== OtherActor (Game|Player|GetPlayerPawn 0))
        (Development|PrintString "Player")
        ;;[0 1 0.09066] Player Hit
        (Utilities|FlowControl|DoOnce false
          (:Completed
            (CallFunction|PlayerHitWidgetFeedbacks)
            (Character|LaunchCharacter (Game|GetPlayerCharacter 0) (Math|Vector|MakeVector (.x _returnvalue_3) (.y _returnvalue_3) (+ (.z _returnvalue_3) 7.5e+02)) false false)
            (Components|Activation|Deactivate (Variables|Default|GetDustMovement))
            (if (<= (Variables|/Game/UI/WBP_Score.WBP_Score_C|GetCurrentScore (Variables|/Game/Blueprints/PC_Test.PC_Test_C|GetScoreWidget (Variables|Default|GetAs%20PC%20Test))) 0.0)
              (CallFunction|PlayerHitNoCoin)
              (else
                (Variables|DecreaseCoin|SetTimesDone 0)
                (bind _returnvalue_4 (Utilities|Time|SetTimerbyEvent (delegate Custom|DecreaseCoinNumber) 0.1 true))
                (Variables|DecreaseCoin|SetDecreaseNumberTimer _returnvalue_4)
                (Class|NiagaraComponent|SetVariableInt _niagaracoinfalloff "Spawn Count" 3)
                (Transformation|SetWorldLocation _niagaracoinfalloff (+ (Transformation|GetActorLocation (Game|GetPlayerCharacter 0)) "0.000000,0.000000,100.000000") false true)
                (Components|Activation|Activate _niagaracoinfalloff false)
                (Audio|PlaySoundatLocation "/Game/Sounds/A_CoinFall_Cue.A_CoinFall_Cue" (Transformation|GetWorldLocation _niagaracoinfalloff) "0, 0, 0" 1.0 1.0 0.0 0 0 0 0)
                (Utilities|FlowControl|DelayUntilNextTick)
                (CallFunction|Reset)
                (Utilities|FlowControl|Delay 1.8)
                (CallFunction|MovementFinished)))))
        (else
          (Development|PrintString "Other")
          ;;[1 0.05756 0] Enviro Hit
          (Components|Activation|Deactivate (Variables|Default|GetDustMovement))
          (Variables|/Script/Engine.MovementComponent|SetVelocity (Variables|/Script/Engine.Character|GetCharacterMovement (Variables|Default|GetAs%20PC%20Test)) "0, 0, 0")
          (Character|LaunchCharacter (* (Math|Vector|NegateVector (Math|Vector|GetForwardVector (Transformation|GetActorRotation))) 3e+03) false false)
          (bind _rotatingenemy (Timeline|Rotate PlayFromStart)
            (:Update
              (Transformation|SetActorRotation (Math|Rotator|MakeRotator _rotatingenemy 0.0 0.0))
              (Utilities|FlowControl|Delay 2.0)
              (bind _rotatingenemy_2 (Timeline|Timeline ReverseFromEnd)
                (:Update
                  (Transformation|SetActorRotation (Math|Rotator|MakeRotator _rotatingenemy_2 0.0 0.0))
                  (CallFunction|MovementFinished))))))))))

(event Custom|MovementFinished
  (bind _returnvalue (Transformation|GetActorLocation))
  (bind _returnvalue_2 (Game|GetPlayerCharacter 0))
  (bind _returnvalue_3 (Transformation|GetActorLocation _returnvalue_2))
  (bind _returnvalue_4 (Math|Rotator|FindLookatRotation _returnvalue _returnvalue_3))
  (Utilities|FlowControl|Delay 5.0)
  (Variables|Default|SetCanDash? true)
  ;[0.2235 0.9103 1] Character Rotates
  (Utilities|FlowControl|DoOnce false) ; enters at Reset
)

(event Custom|Reset
  (bind _capsulecomponent (Variables|Collision|GetCapsuleComponent))
  (bind _niagaracoinfalloff (Variables|Default|GetNiagaraCoinFallOff))
  (bind _returnvalue (Transformation|GetWorldRotation _capsulecomponent))
  (bind _returnvalue_2 (Math|Vector|GetForwardVector _returnvalue))
  (bind _returnvalue_3 (* _returnvalue_2 1e+03))
  ;[1 0.889 0.04791] Hits something
  ;;[0 1 0.09066] Player Hit
  (Utilities|FlowControl|DoOnce false) ; enters at Reset
)

(event Custom|PlayerHitWidgetFeedbacks
  ;[1 1 1] Called when the player gets hit
  (Default|PlayerHit (Variables|Default|GetAs%20PC%20Test)))

(event Custom|PlayerHitNoCoin
  ;[1 1 1] Called when the Player is "Dying"
  (Default|NoCoinLeft (Variables|Default|GetAs%20PC%20Test)))

(event Custom|DecreaseCoinNumber
  (bind _as_pc_test (Variables|Default|GetAs%20PC%20Test))
  (bind _scorewidget (Variables|/Game/Blueprints/PC_Test.PC_Test_C|GetScoreWidget _as_pc_test))
  ;[1 0.889 0.04791] Hits something
  ;;[0 1 0.09066] Player Hit
  ;;;[0.6985 1 0] Decreasing the Coin Number Smoothly
  (if (== (Variables|DecreaseCoin|GetTimesDone) 3)
    (Utilities|Time|ClearandInvalidateTimerbyHandle (Variables|DecreaseCoin|GetDecreaseNumberTimer))
    (else
      (Variables|/Game/UI/WBP_Score.WBP_Score_C|SetCurrentScore _scorewidget (Math|Float|Clamp(Float) (- (Variables|/Game/UI/WBP_Score.WBP_Score_C|GetCurrentScore _scorewidget) 1.0) 0.0 1e+02))
      (Variables|DecreaseCoin|SetTimesDone (+ (Variables|DecreaseCoin|GetTimesDone) 1))
      (Default|DecreaseNumber (Variables|/Game/Blueprints/PC_Test.PC_Test_C|GetScoreWidget (Variables|Default|GetAs%20PC%20Test))))))

(event EventBeginPlay
  ;[1 1 1 0.3] Begin
  (bind _aspc_test (Utilities|Casting|CastToPC_Test (Game|GetPlayerCharacter 0)))
  (Variables|Default|SetAs%20PC%20Test _aspc_test)
  (Niagara|SetNiagaraVariable(Object) (Variables|Default|GetNiagaraCoinFallOff) "BP_callback" self))

(event EventParticleData
  (params (Data :type Array%20of%20Basic%20Particle%20Data%20Structures) (NiagaraSystem :type Niagara%20System%20Object%20Reference) (SimulationPositionOffset :type Vector%20%28by%20ref%29 :default "0, 0, 0"))
  ;[0 1 0.09066] On CoinFallOff particles death
  (for _array_element Data
    (Game|SpawnActorfromClass "/Game/Blueprints/GPE/BP_Coin.BP_Coin_C" (Math|Conversions|ToTransform(Vector) (.Position (Utilities|Struct|BreakBasicParticleData _array_element))) "AdjustIfPossibleButAlwaysSpawn" "MultiplyWithRoot" 0 0)))

(event EventTick
  (params (DeltaSeconds :type Float%20%28single-precision%29))
  (bind _returnvalue (Transformation|GetActorLocation))
  (bind _returnvalue_2 (Game|GetPlayerCharacter 0))
  (bind _returnvalue_3 (Transformation|GetActorLocation _returnvalue_2))
  (bind _returnvalue_4 (Math|Rotator|FindLookatRotation _returnvalue _returnvalue_3))
  (if (Variables|Default|GetPlayerDetected?)
    (Development|PrintString "Player Detected" true true "(R=0.450309,G=0.000000,B=1.000000,A=1.000000)" 2.0 "333")
    (Utilities|FlowControl|Sequence
      (:then_0
        ;[0.2235 0.9103 1] Character Rotates
        (Utilities|FlowControl|DoOnce false
          (:Completed
            (Variables|Default|SetPlayerPosition (Transformation|GetActorLocation (Game|GetPlayerCharacter 0)))
            (Transformation|SetActorRotation (Math|Rotator|MakeRotator (.roll _returnvalue_4) 0.0 (.yaw _returnvalue_4))))))
      (:then_1
        (if (Variables|Default|GetCanDash?)
          (Rendering|SetVisibility (Variables|Default|GetExclamationMark) false false)
          ;[0.141 0.4403 1] Character Moves towards the Player
          (Character|LaunchCharacter (* (Math|Vector|GetForwardVector (Transformation|GetActorRotation)) 75.0) false false)
          (Components|Activation|Activate (Variables|Default|GetDustMovement) false)
          (Utilities|FlowControl|Delay (Variables|Default|GetDashDuration))
          (Variables|Default|SetCanDash? false))))))

(fn ConstructionScript)