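; PC_Test is a test character Blueprint that tunes jump feel, with debug prints for vertical speed, gravity scale, apex and landing.
; Tick zeroes slow upward velocity to cut the rise short, reusing cached horizontal velocity.
; Reaching the jump apex raises gravity for a faster fall.
; Landing restores gravity, sets jump velocity, plays controller force feedback and spawns a landing Niagara effect.
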(event Custom|OnReachedJumpApex_Event
  (Development|PrintString "APEX" true true "(R=1.000000,G=0.083818,B=0.000000,A=1.000000)" 2.0 "8888")
  (Variables|/Script/Engine.CharacterMovementComponent|SetGravityScale (Variables|Character|GetCharacterMovement) 2.5))

(event EventBeginPlay
  (EventDispatchers|BindEventtoOnReachedJumpApex (delegate Custom|OnReachedJumpApex_Event)))

(event EventOnLanded
  (params (Hit :type Hit%20Result%20Structure%20%28by%20ref%29))
  (bind _charactermovement (Variables|Character|GetCharacterMovement))
  (Development|PrintString "Landed" true true "(R=0.000000,G=0.660000,B=1.000000,A=1.000000)" 2.0 "456")
  (Variables|/Script/Engine.CharacterMovementComponent|SetGravityScale _charactermovement 1.0)
  (Variables|/Script/Engine.CharacterMovementComponent|SetJumpZVelocity _charactermovement 6.5e+02)
  (Game|Feedback|ClientPlayForceFeedback (Game|GetPlayerController 0) "/Game/Haptic/FFE_Landing.FFE_Landing" "None" false false false)
  (Niagara|SpawnSystematLocation "/Game/NS/NS_Land.NS_Land" (Transformation|GetWorldLocation (Variables|Default|GetVFX))))

(event EventTick
  (params (DeltaSeconds :type Float%20%28single-precision%29))
  (bind _returnvalue (Transformation|GetVelocity))
  (bind _returnvalue_2 (Transformation|GetVelocity))
  (bind _z (Math|Vector|BreakVector _returnvalue))
  (bind (_x _y) (Math|Vector|BreakVector _returnvalue_2))
  (Utilities|FlowControl|Sequence
    (:then_0
      (Development|PrintString (Utilities|String|ToString(Float) _z) true true "(R=1.000000,G=0.774798,B=0.000000,A=1.000000)" 2.0 "1")
      (if (and (<= _z 1.2e+02) (not (<= _z 0.0)))
        (Variables|/Script/Engine.MovementComponent|SetVelocity (Variables|Character|GetCharacterMovement) (Math|Vector|MakeVector (Variables|Default|GetVelocity%20X) (Variables|Default|GetVelocity%20Y) 0.0))))
    (:then_1
      (Variables|Default|SetVelocity%20Y _y)
      (Variables|Default|SetVelocity%20X _x))
    (:then_2
      (Development|PrintString (Utilities|String|ToString(Float) (Variables|/Script/Engine.CharacterMovementComponent|GetGravityScale (Variables|Character|GetCharacterMovement))) true true "(R=0.000000,G=0.660000,B=1.000000,A=1.000000)" 2.0 "1443"))))

(fn ConstructionScript)