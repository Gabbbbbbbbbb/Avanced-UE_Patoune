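; GI_Save saves the player's coin totals, TotalCoin and OwnedCoin, into a GS_Save save game under a given slot name.
; If the slot exists, Saving casts the current GS reference, loads the slot into GS, then writes and saves the cast object, stopping if that cast fails.
; Otherwise it creates a new GS_Save, fills and saves it, with a debug print on either path.
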(fn Saving
  (params (SaveName :type String) (GI_TotalCoin :type Float%20%28double-precision%29) (GI_OwnedCoin :type Float%20%28double-precision%29))
  (bind _output_get (Variables|Default|SetSave%20Name SaveName))
  (Variables|Default|SetGI%20Total%20Coin GI_TotalCoin)
  (Variables|Default|SetGI%20Owned%20Coin GI_OwnedCoin)
  (bind _returnvalue (SaveGame|DoesSaveGameExist _output_get))
  (if _returnvalue
    ;[1 1 1] Loading then saving
    (bind _asgs_save (Utilities|Casting|CastToGS_Save (Variables|Default|GetGS)))
    (bind _returnvalue_2 (SaveGame|LoadGamefromSlot (Variables|Default|GetSave%20Name)))
    (Variables|Default|SetGS _returnvalue_2)
    (Variables|/Game/Blueprints/Save/GS_Save.GS_Save_C|SetTotalCoin _asgs_save (Variables|Default|GetGI%20Total%20Coin))
    (Variables|/Game/Blueprints/Save/GS_Save.GS_Save_C|SetOwnedCoin _asgs_save (Variables|Default|GetGI%20Owned%20Coin))
    (SaveGame|SaveGametoSlot _asgs_save (Variables|Default|GetSave%20Name))
    (Development|PrintString "done")
    (else
      ;[1 1 1] Creating save + saving
      (bind _returnvalue_3 (SaveGame|CreateSaveGameObject "/Game/Blueprints/Save/GS_Save.GS_Save_C"))
      (Variables|Default|SetGS _returnvalue_3)
      (Variables|/Game/Blueprints/Save/GS_Save.GS_Save_C|SetOwnedCoin _returnvalue_3 (Variables|Default|GetGI%20Owned%20Coin))
      (Variables|/Game/Blueprints/Save/GS_Save.GS_Save_C|SetTotalCoin _returnvalue_3 (Variables|Default|GetGI%20Total%20Coin))
      (SaveGame|SaveGametoSlot _returnvalue_3 (Variables|Default|GetSave%20Name))
      (Development|PrintString "Save Created" true true "(R=1.000000,G=0.606406,B=0.000000,A=1.000000)"))))