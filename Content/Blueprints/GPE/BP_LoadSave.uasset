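; BP_LoadSave is a gameplay Blueprint that restores the player's saved coin progress when play begins.
; BeginPlay calls Load, which waits one tick, then loads the GS_Save object from the SaveName slot if it exists.
; It passes the saved total and owned coin values to LoadCoin on the PC_Test player pawn.
; Despite its name, it contains no saving logic.
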(event Custom|Load
  (Utilities|FlowControl|DelayUntilNextTick)
  (bind _returnvalue (SaveGame|DoesSaveGameExist (Variables|Default|GetSaveName)))
  (if _returnvalue
    (bind _returnvalue_2 (SaveGame|LoadGamefromSlot (Variables|Default|GetSaveName)))
    (bind _asgs_save (Utilities|Casting|CastToGS_Save _returnvalue_2))
    (Variables|Default|SetAs%20GS%20Save _asgs_save)
    (bind _aspc_test (Utilities|Casting|CastToPC_Test (Game|Player|GetPlayerPawn 0)))
    (Default|LoadCoin _aspc_test (Variables|/Game/Blueprints/Save/GS_Save.GS_Save_C|GetTotalCoin (Variables|Default|GetAs%20GS%20Save)) (Variables|/Game/Blueprints/Save/GS_Save.GS_Save_C|GetOwnedCoin (Variables|Default|GetAs%20GS%20Save)))))

(event EventBeginPlay
  (CallFunction|Load))

(fn ConstructionScript)